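; Damage zone actor that drains the first-person player's health while they stand inside its box.
; Box begin and end overlap events cache the FirstPersonCharacter and toggle an overlap flag.
; While the flag is set, Tick subtracts DamageHit every frame without delta-time scaling, clamps health at zero, and updates the player's HP widget.
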(event OnComponentBeginOverlap(Box)
  (params (OverlappedComponent :type Primitive%20Component%20Object%20Reference) (OtherActor :type Actor%20Object%20Reference) (OtherComp :type Primitive%20Component%20Object%20Reference) (OtherBodyIndex :type Integer) (bFromSweep :type Boolean) (SweepResult :type Hit%20Result%20Structure%20%28by%20ref%29))
  (bind _asfirst_person_character (Utilities|Casting|CastToFirstPersonCharacter OtherActor))
  (Variables|Default|SetFPC _asfirst_person_character)
  (Variables|Default|SetIsPlayeroverLap true))

(event OnComponentEndOverlap(Box)
  (params (OverlappedComponent :type Primitive%20Component%20Object%20Reference) (OtherActor :type Actor%20Object%20Reference) (OtherComp :type Primitive%20Component%20Object%20Reference) (OtherBodyIndex :type Integer))
  (bind _asfirst_person_character (Utilities|Casting|CastToFirstPersonCharacter OtherActor))
  (Variables|Default|SetFPC _asfirst_person_character)
  (Variables|Default|SetIsPlayeroverLap false))

(event EventTick
  (params (DeltaSeconds :type Float%20%28single-precision%29))
  (bind _fpc (Variables|Default|GetFPC))
  (bind _ui_playerhp (Variables|/Game/FirstPersonCPP/Blueprints/FirstPersonCharacter.FirstPersonCharacter_C|GetUI_PlayerHP _fpc))
  (if (Variables|Default|GetIsPlayeroverLap)
    (if (> (- (Variables|/Game/FirstPersonCPP/Blueprints/FirstPersonCharacter.FirstPersonCharacter_C|GetCurrentHealth _fpc) (Variables|Default|GetDamageHit)) 0.0)
      (bind _output_get (Variables|/Game/FirstPersonCPP/Blueprints/FirstPersonCharacter.FirstPersonCharacter_C|SetCurrentHealth _fpc (- (Variables|/Game/FirstPersonCPP/Blueprints/FirstPersonCharacter.FirstPersonCharacter_C|GetCurrentHealth _fpc) (Variables|Default|GetDamageHit))))
      (Variables|/Game/GG/UI/UI_PlayerHP.UI_PlayerHP_C|SetCurrentHP _ui_playerhp _output_get)
      (else
        (bind _output_get_2 (Variables|/Game/FirstPersonCPP/Blueprints/FirstPersonCharacter.FirstPersonCharacter_C|SetCurrentHealth _fpc 0.0))
        (Variables|/Game/GG/UI/UI_PlayerHP.UI_PlayerHP_C|SetCurrentHP _ui_playerhp _output_get_2)))
    (Default|UpdateHP _ui_playerhp)))

(fn ConstructionScript)